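; BP_Coding is a practice Blueprint for basic arithmetic functions, loops and printing, in a folder named MyFirstBluePrint.
; BeginPlay prints the result of Minus, though that function's graph holds only an unused subtraction node.
; Disconnected chains, which never run, call Plus and Multiply and sum the even numbers of a loop into Number.
; The construction script, overlap and Tick events are empty.
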(event Collision|EventActorBeginOverlap
  (params (OtherActor :type Actor%20Object%20Reference)))

(event EventTick
  (params (DeltaSeconds :type Float%20%28single-precision%29)))

(event EventBeginPlay
  (Development|PrintString (Utilities|String|ToString(Integer) (Utilities|Minus 5 2))))

(fn ConstructionScript)

(fn Plus
  (params (a :type Integer) (b :type Integer))
  (return (+ a b)))

(fn Multiply
  (params (a :type Integer) (b :type Integer))
  (return (* a b)))